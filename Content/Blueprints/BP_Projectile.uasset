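; BP_Projectile is a projectile actor that damages BP_EnemyBase enemies and destroys itself on impact.
; Every tick it runs a Visibility line trace from its location to its EndTrace component, with one-frame debug drawing, and destroys itself without dealing damage on any hit.
; HitBox overlaps with an enemy store the reference, apply BaseDamage, then destroy the projectile; other overlapping actors are ignored.
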(event OnComponentBeginOverlap(HitBox)
  (params (OverlappedComponent :type Primitive%20Component%20Object%20Reference) (OtherActor :type Actor%20Object%20Reference) (OtherComp :type Primitive%20Component%20Object%20Reference) (OtherBodyIndex :type Integer) (bFromSweep :type Boolean) (SweepResult :type Hit%20Result%20Structure%20%28by%20ref%29))
  (bind _asbp_enemy_base (Utilities|Casting|CastToBP_EnemyBase OtherActor))
  (bind _output_get (Variables|Default|SetEnemyRef _asbp_enemy_base))
  (Game|Damage|ApplyDamage _output_get (Variables|Default|GetBase%20Damage) 0 0)
  (Actor|DestroyActor))

(event EventBeginPlay)

(event Collision|EventActorBeginOverlap
  (params (OtherActor :type Actor%20Object%20Reference)))

(event EventTick
  (params (DeltaSeconds :type Float%20%28single-precision%29))
  (bind _returnvalue (Collision|LineTraceByChannel (Transformation|GetActorLocation) (Transformation|GetWorldLocation (Variables|Default|GetEndTrace)) "TraceTypeQuery1" false 0 "ForOneFrame"))
  (if _returnvalue
    (Actor|DestroyActor)))

(fn ConstructionScript)