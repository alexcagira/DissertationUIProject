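; Main player controller that holds the player's display and accessibility settings: heart health bar, coins bar, shadows, font and dyslexia options.
; On BeginPlay it loads them from the "Settings" save slot, or creates a default BP_SavedConfig save if none exists.
; Getters expose each value, and setters write all values back through SaveData.
; The font setter instead broadcasts OnFontChange without saving.
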(event Custom|SaveData
  (bind _returnvalue (SaveGame|LoadGamefromSlot "Settings"))
  (bind _asbp_saved_config (Utilities|Casting|CastToBP_SavedConfig _returnvalue))
  (Variables|/Game/Blueprints/Data/BP_SavedConfig.BP_SavedConfig_C|SetIsHeartBar _asbp_saved_config (Variables|Default|GetIsHeartBar))
  (Variables|/Game/Blueprints/Data/BP_SavedConfig.BP_SavedConfig_C|SetFontIndex _asbp_saved_config (Variables|Default|GetFontIndex))
  (Variables|/Game/Blueprints/Data/BP_SavedConfig.BP_SavedConfig_C|SetDyslexiaBold _asbp_saved_config (Variables|Default|GetDyslexiaBold))
  (Variables|/Game/Blueprints/Data/BP_SavedConfig.BP_SavedConfig_C|SetDyslexiaNormal _asbp_saved_config (Variables|Default|GetDyslexiaNormal))
  (Variables|/Game/Blueprints/Data/BP_SavedConfig.BP_SavedConfig_C|SetIsCoinsBar _asbp_saved_config (Variables|Default|GetIsCoinsBar))
  (Variables|/Game/Blueprints/Data/BP_SavedConfig.BP_SavedConfig_C|SetIsShadows _asbp_saved_config (Variables|Default|GetIsShadows))
  (SaveGame|SaveGametoSlot _asbp_saved_config "Settings"))

(event EventSetDyslexiaBold
  (params (NewDyslexiaBold :type Boolean))
  (Variables|Default|SetDyslexiaBold NewDyslexiaBold)
  (CallFunction|SaveData))

(event EventSetDyslexiaNormal
  (params (NewDyslexiaNormal :type Boolean))
  (Variables|Default|SetDyslexiaNormal NewDyslexiaNormal)
  (CallFunction|SaveData))

(event EventSetCurrentFontIndex
  (params (NewFontIndex :type Integer))
  (bind _output_get (Variables|Default|SetFontIndex NewFontIndex))
  (Default|CallOnFontChange _output_get))

(event EventSetHeartHealthBar
  (params (NewIsHeartBar :type Boolean))
  (Variables|Default|SetIsHeartBar NewIsHeartBar)
  (CallFunction|SaveData))

(event EventBeginPlay
  (bind _returnvalue (SaveGame|DoesSaveGameExist "Settings"))
  (if _returnvalue
    (bind _returnvalue_2 (SaveGame|LoadGamefromSlot "Settings"))
    (bind _asbp_saved_config (Utilities|Casting|CastToBP_SavedConfig _returnvalue_2))
    (Variables|Default|SetIsHeartBar (Variables|/Game/Blueprints/Data/BP_SavedConfig.BP_SavedConfig_C|GetIsHeartBar _asbp_saved_config))
    (Variables|Default|SetFontIndex (Variables|/Game/Blueprints/Data/BP_SavedConfig.BP_SavedConfig_C|GetFontIndex _asbp_saved_config))
    (Variables|Default|SetDyslexiaBold (Variables|/Game/Blueprints/Data/BP_SavedConfig.BP_SavedConfig_C|GetDyslexiaBold _asbp_saved_config))
    (Variables|Default|SetDyslexiaNormal (Variables|/Game/Blueprints/Data/BP_SavedConfig.BP_SavedConfig_C|GetDyslexiaNormal _asbp_saved_config))
    (Variables|Default|SetIsCoinsBar (Variables|/Game/Blueprints/Data/BP_SavedConfig.BP_SavedConfig_C|GetIsCoinsBar _asbp_saved_config))
    (Variables|Default|SetIsShadows (Variables|/Game/Blueprints/Data/BP_SavedConfig.BP_SavedConfig_C|GetIsShadows _asbp_saved_config))
    (else
      (bind _returnvalue_3 (SaveGame|CreateSaveGameObject "/Game/Blueprints/Data/BP_SavedConfig.BP_SavedConfig_C"))
      (SaveGame|SaveGametoSlot _returnvalue_3 "Settings"))))

(event EventSetCoinsBar
  (params (NewCoinsBar :type Boolean))
  (Variables|Default|SetIsCoinsBar NewCoinsBar)
  (CallFunction|SaveData))

(event EventSetShadows
  (params (NewIsShadows :type Boolean))
  (Variables|Default|SetIsShadows NewIsShadows)
  (CallFunction|SaveData))

(fn ConstructionScript)

(fn GetCoinsBar
  (return (Variables|Default|GetIsCoinsBar)))

(fn GetCurrentFontIndex
  (return (Variables|Default|GetFontIndex)))

(fn GetDyslexiaBold
  (return (Variables|Default|GetDyslexiaBold)))

(fn GetDyslexiaNormal
  (return (Variables|Default|GetDyslexiaNormal)))

(fn GetHeartHealthBar
  (return (Variables|Default|GetIsHeartBar)))

(fn GetReferencetoSelf
  (return self))

(fn GetShadows
  (return (Variables|Default|GetIsShadows)))