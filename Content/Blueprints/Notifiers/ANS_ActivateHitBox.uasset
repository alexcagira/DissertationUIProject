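; Animation notify state for Paper2D flipbook animations that opens the player's attack hit box during a window of frames.
; On begin it casts the owning paper character to BP_Player and sets its HitBox to query-only collision.
; On end it turns the HitBox collision off, and it displays as "ActivateHitBox".
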(event EventOnNotifyBegin
  (params (OwningInstance :type Paper%20ZD%20Anim%20Instance%20Object%20Reference))
  (bind _asbp_player (Utilities|Casting|CastToBP_Player (Class|PaperZDAnimInstance|GetPaperCharacter OwningInstance)))
  (Collision|SetCollisionEnabled (Variables|/Game/Blueprints/BP_Player.BP_Player_C|GetHitBox _asbp_player) "QueryOnly"))

(event EventOnNotifyEnd
  (params (OwningInstance :type Paper%20ZD%20Anim%20Instance%20Object%20Reference))
  (bind _asbp_player (Utilities|Casting|CastToBP_Player (Class|PaperZDAnimInstance|GetPaperCharacter OwningInstance)))
  (Collision|SetCollisionEnabled (Variables|/Game/Blueprints/BP_Player.BP_Player_C|GetHitBox _asbp_player) "NoCollision"))

(fn GetDisplayName
  (return "ActivateHitBox"))