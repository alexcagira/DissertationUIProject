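; BP_BaseTrap is a base environment trap that damages the player on contact and sends them back to their last platform.
; BeginPlay caches the player character as BP_Player, and the HitBox overlap reacts only to that actor.
; On overlap it applies BaseDamage, then teleports the player to the location and rotation stored in their LastPlatformPos.
; The construction script sizes the HitBox from the BoxExtent variable.
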(event OnComponentBeginOverlap(HitBox)
  (params (OverlappedComponent :type Primitive%20Component%20Object%20Reference) (OtherActor :type Actor%20Object%20Reference) (OtherComp :type Primitive%20Component%20Object%20Reference) (OtherBodyIndex :type Integer) (bFromSweep :type Boolean) (SweepResult :type Hit%20Result%20Structure%20%28by%20ref%29))
  (bind _playerref (Variables|Default|GetPlayerRef))
  (bind _lastplatformpos (Variables|/Game/Blueprints/BP_Player.BP_Player_C|GetLastPlatformPos _playerref))
  (if (== OtherActor (Variables|Default|GetPlayerRef))
    (Game|Damage|ApplyDamage (Variables|Default|GetPlayerRef) (Variables|Default|GetBase%20Damage) 0 0)
    (Transformation|SetActorTransform (Variables|Default|GetPlayerRef) (Math|Transform|MakeTransform (.location _lastplatformpos) (.rotation _lastplatformpos) "1.000000,1.000000,1.000000"))))

(event EventBeginPlay
  (bind _asbp_player (Utilities|Casting|CastToBP_Player (Game|GetPlayerCharacter 0)))
  (Variables|Default|SetPlayerRef _asbp_player))

(fn ConstructionScript
  (Components|Box|SetBoxExtent (Variables|Default|GetHitBox) (Variables|Default|GetBox%20Extent) true))