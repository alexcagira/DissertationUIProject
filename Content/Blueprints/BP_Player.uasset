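; Player character for a side-scrolling PaperZD game, handling Enhanced Input movement, jumping, melee and shooting animations, coin pickups and a pause menu.
; Attack animation overrides gate further attacks, while HitBox overlaps damage BP_EnemyBase actors.
; Damage updates the MainHUD, then either launches the player into timed hit stun and invulnerability or plays death and reloads the level.
; The menu pauses through global time dilation, and velocity direction sets facing.
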(event OnComponentBeginOverlap(CapsuleComponent)
  (params (OverlappedComponent :type Primitive%20Component%20Object%20Reference) (OtherActor :type Actor%20Object%20Reference) (OtherComp :type Primitive%20Component%20Object%20Reference) (OtherBodyIndex :type Integer) (bFromSweep :type Boolean) (SweepResult :type Hit%20Result%20Structure%20%28by%20ref%29))
  (if (Utilities|DoesObjectImplementInterface OtherActor "/Game/Blueprints/Interface/BPi_Collectable.BPi_Collectable_C")
    (Utilities|FlowControl|Sequence
      (:then_0
        (if (Actor|ActorHasTag OtherActor "Coin")
          (bind _result (Math|Integer|IncrementInt (Variables|Default|GetCoinsObtain))
            (:%20%20
              (Default|UpdateCoinCount (Variables|Default|GetMainHUD) _result)))))
      (:then_1
        (Class|BPiCollectable|PickUp(Message) OtherActor)))))

(event OnComponentBeginOverlap(HitBox)
  (params (OverlappedComponent :type Primitive%20Component%20Object%20Reference) (OtherActor :type Actor%20Object%20Reference) (OtherComp :type Primitive%20Component%20Object%20Reference) (OtherBodyIndex :type Integer) (bFromSweep :type Boolean) (SweepResult :type Hit%20Result%20Structure%20%28by%20ref%29))
  (bind _asbp_enemy_base (Utilities|Casting|CastToBP_EnemyBase OtherActor))
  (Game|Damage|ApplyDamage _asbp_enemy_base (Variables|Default|GetCurrentDamage) 0 0))

(event Custom|HitStunRecovery
  ;[1 1 1] Damage System
  (CallFunction|AddPlayerInput)
  (Variables|/Script/Engine.CharacterMovementComponent|SetFallingLateralFriction (Variables|Character|GetCharacterMovement) (Variables|Default|GetDefaultLateralFriction))
  (Utilities|Time|SetTimerbyEvent (EventDispatchers|CreateEvent :!event Custom|InvulnerabilityRecovery) (Variables|Default|GetInvulnerabilityTime)))

(event Custom|InvulnerabilityRecovery
  ;[1 1 1] Damage System
  (Collision|SetCollisionResponsetoChannel (Variables|Default|GetCapsuleComponent) "ECC_GameTraceChannel1" "ECR_Overlap"))

(event Custom|Death
  (bind _returnvalue (Game|GetCurrentLevelName true))
  (Game|OpenLevel(byName) (Utilities|String|StringToName _returnvalue)))

(event Input|EnhancedActionEvents|EnhancedInputActionIA_Jump
  (params (ActionValue :type Boolean) (ElapsedSeconds :type Float%20%28double-precision%29) (TriggeredSeconds :type Float%20%28double-precision%29) (InputAction :type Input%20Action%20Object%20Reference :default "/Game/Blueprints/Inputs/Actions/IA_Jump.IA_Jump"))
  (:Started
    (if (not (Variables|Default|GetIsUIOn))
      (Character|Jump))))

(event Input|EnhancedActionEvents|EnhancedInputActionIA_Move
  (params (ActionValue :type Float%20%28double-precision%29) (ElapsedSeconds :type Float%20%28double-precision%29) (TriggeredSeconds :type Float%20%28double-precision%29) (InputAction :type Input%20Action%20Object%20Reference :default "/Game/Blueprints/Inputs/Actions/IA_Move.IA_Move"))
  (Pawn|Input|AddMovementInput "1.000000,0.000000,0.000000" ActionValue false))

(event Input|EnhancedActionEvents|EnhancedInputActionIA_Attack
  (params (ActionValue :type Boolean) (ElapsedSeconds :type Float%20%28double-precision%29) (TriggeredSeconds :type Float%20%28double-precision%29) (InputAction :type Input%20Action%20Object%20Reference :default "/Game/Blueprints/Inputs/Actions/IA_Attack.IA_Attack"))
  (:Started
    (if (Variables|Default|GetCanAttack)
      (|PlayAnimationOverridewithCallbacks (Class|PaperZDCharacter|GetAnimInstance) "/Game/Blueprints/Animations/AnimSequences/PlayerAttack.PlayerAttack" "DefaultSlot" 1.0 0.0
        (:then
          (Variables|Default|SetCanAttack false))
        (:OnCompleted
          (Variables|Default|SetCanAttack true :!label _label))
        (:OnCancelled
          (goto _label))))))

(event Input|EnhancedActionEvents|EnhancedInputActionIA_Shoot
  (params (ActionValue :type Boolean) (ElapsedSeconds :type Float%20%28double-precision%29) (TriggeredSeconds :type Float%20%28double-precision%29) (InputAction :type Input%20Action%20Object%20Reference :default "/Game/Blueprints/Inputs/Actions/IA_Shoot.IA_Shoot"))
  (:Started
    (if (Variables|Default|GetCanAttack)
      (|PlayAnimationOverridewithCallbacks (Class|PaperZDCharacter|GetAnimInstance) "/Game/Blueprints/Animations/AnimSequences/PlayerShot.PlayerShot" "DefaultSlot" 1.0 0.0
        (:then
          (Variables|Default|SetCanAttack false))
        (:OnCompleted
          (Variables|Default|SetCanAttack true :!label _label))
        (:OnCancelled
          (goto _label))))))

(event Input|EnhancedActionEvents|EnhancedInputActionIA_Menu
  (params (ActionValue :type Boolean) (ElapsedSeconds :type Float%20%28double-precision%29) (TriggeredSeconds :type Float%20%28double-precision%29) (InputAction :type Input%20Action%20Object%20Reference :default "/Game/Blueprints/Inputs/Actions/IA_Menu.IA_Menu"))
  (bind _returnvalue (Game|GetPlayerController 0))
  (bind _mainhud (Variables|Default|GetMainHUD))
  (:Started
    (Utilities|FlowControl|FlipFlop
      (:A
        (Default|CloseMenu _mainhud)
        (Utilities|Time|SetGlobalTimeDilation 1.0)
        (Variables|Default|SetIsUIOn false))
      (:B
        (Default|OpenMenu _mainhud)
        (Input|SetInputModeGameandUI _returnvalue (Variables|Default|GetMainHUD) "DoNotLock" true false)
        (Variables|/Script/Engine.PlayerController|SetbShowMouseCursor _returnvalue true)
        (Utilities|Time|SetGlobalTimeDilation 0.0)
        (Variables|Default|SetIsUIOn true)))))

(event EventBeginPlay
  (Input|SetInputModeGameOnly (Game|GetPlayerController 0) false)
  (Audio|PlaySound2D "/Game/Sounds/LevelMusic_Cue.LevelMusic_Cue" 1.0 1.0 0.0 0 0)
  (bind _returnvalue (UserInterface|CreateWidget "/Game/Blueprints/Widgets/WD_MainHUD.WD_MainHUD_C"))
  (bind _output_get (Variables|Default|SetMainHUD _returnvalue))
  (UserInterface|Viewport|AddtoViewport _output_get 0)
  (CallFunction|AddPlayerInput)
  (Variables|Default|SetDefaultLateralFriction (Variables|/Script/Engine.CharacterMovementComponent|GetFallingLateralFriction (Variables|Character|GetCharacterMovement)))
  (Variables|Default|SetLastPlatformPos (Variables|Default|GetLastPlatformPos)))

(event Collision|EventActorBeginOverlap
  (params (OtherActor :type Actor%20Object%20Reference)))

(event EventTick
  (params (DeltaSeconds :type Float%20%28single-precision%29))
  (Math|Float|CompareFloat (.x (Transformation|GetVelocity)) 0.0
    (:>
      (Pawn|SetControlRotation (Game|GetPlayerController 0) (Math|Rotator|MakeRotator 0.0 0.0 0.0)))
    (:<
      (Pawn|SetControlRotation (Game|GetPlayerController 0) (Math|Rotator|MakeRotator 0.0 0.0 1.8e+02)))))

(event Game|Damage|EventAnyDamage
  (params (Damage :type Float%20%28single-precision%29) (DamageType :type Damage%20Type%20Object%20Reference) (InstigatedBy :type Controller%20Object%20Reference) (DamageCauser :type Actor%20Object%20Reference))
  ;[1 1 1] Check for Player Life Points
  (bind _output_get (Variables|Default|SetCurrentHealth (Math|Float|Clamp(Float) (- (Variables|Default|GetCurrentHealth) Damage) 0.0 (- (Variables|Default|GetCurrentHealth) Damage))))
  (Default|UpdateHPBar (Variables|Default|GetMainHUD) _output_get)
  ;[1 1 1] Damage System
  (if (== _output_get 0.0)
    (Variables|Default|SetIsDead true)
    (if (Variables|Default|GetIsDead)
      (CallFunction|RemovePlayerInput)
      (Class|PaperZDAnimInstance|JumptoNode (Class|PaperZDCharacter|GetAnimInstance) "JumpDead" "None")
      (Utilities|FlowControl|Delay 1.0)
      (CallFunction|Death))
    (else
      (CallFunction|ReceiveDamage))))

(event EventImpact
  (params (Damage :type Float%20%28double-precision%29))
  (Game|Damage|ApplyDamage self Damage 0 0))

(fn ConstructionScript
  (bind _output_get (Variables|Default|SetCurrentHealth (Variables|Default|GetMaxHealth)))
  (Variables|Default|SetCurrentDamage (Variables|Default|GetMaxDamage))
  (Development|PrintString (Utilities|String|ToString(Float) _output_get)))

(fn AddPlayerInput
  (bind _asplayer_controller (Utilities|Casting|CastToPlayerController (Pawn|GetController)))
  (Input|AddMappingContext (PlayerController|LocalPlayerSubsystems|GetEnhancedInputLocalPlayerSubsystem _asplayer_controller) "/Game/Blueprints/Inputs/IMC_PlayerInput.IMC_PlayerInput" 0 "(bIgnoreAllPressedKeysUntilRelease=True,bForceImmediately=False,bNotifyUserSettings=False)"))

(fn RemovePlayerInput
  (bind _asplayer_controller (Utilities|Casting|CastToPlayerController (Pawn|GetController)))
  (Input|RemoveMappingContext (PlayerController|LocalPlayerSubsystems|GetEnhancedInputLocalPlayerSubsystem _asplayer_controller) "/Game/Blueprints/Inputs/IMC_PlayerInput.IMC_PlayerInput" "(bIgnoreAllPressedKeysUntilRelease=True,bForceImmediately=False,bNotifyUserSettings=False)"))

(fn ReceiveDamage
  (Collision|SetCollisionResponsetoChannel (Variables|Default|GetCapsuleComponent) "ECC_GameTraceChannel1" "ECR_Ignore")
  (Variables|/Script/Engine.CharacterMovementComponent|SetFallingLateralFriction (Variables|Character|GetCharacterMovement) 0.0)
  (Character|LaunchCharacter (+ (* (Transformation|GetActorForwardVector) (Variables|Default|GetLateralLaunchVelocity)) (Variables|Default|GetUpwardsLaunchVelocity)) true true)
  (CallFunction|RemovePlayerInput)
  (Utilities|Time|SetTimerbyEvent (EventDispatchers|CreateEvent :!event Custom|HitStunRecovery) (Variables|Default|GetHitStunTime)))

(fn GetMainUI
  (return (Variables|Default|GetMainHUD)))