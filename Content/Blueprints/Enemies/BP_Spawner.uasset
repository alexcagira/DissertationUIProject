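; BP_Spawner is a trigger-box actor that spawns an enemy as the player leaves its volume.
; Player entry arms CanSpawn if EnemyRef1 is invalid; exit disarms it and spawns EnemyToSpawn1 at SpawnPos1.
; EnemyRef1 is set to None after spawning rather than to the new enemy, so spawned enemies do not block re-arming.
; The construction script applies the configurable box extent and spawn location.
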(event OnComponentBeginOverlap(Box)
  (params (OverlappedComponent :type Primitive%20Component%20Object%20Reference) (OtherActor :type Actor%20Object%20Reference) (OtherComp :type Primitive%20Component%20Object%20Reference) (OtherBodyIndex :type Integer) (bFromSweep :type Boolean) (SweepResult :type Hit%20Result%20Structure%20%28by%20ref%29))
  (if (== OtherActor (Variables|Default|GetPlayerRef))
    (Utilities|IsValid (Variables|Default|GetEnemyRef1)
      (:Is%20Not%20Valid
        (Variables|Default|SetCanSpawn true)))))

(event OnComponentEndOverlap(Box)
  (params (OverlappedComponent :type Primitive%20Component%20Object%20Reference) (OtherActor :type Actor%20Object%20Reference) (OtherComp :type Primitive%20Component%20Object%20Reference) (OtherBodyIndex :type Integer))
  (if (and (== OtherActor (Variables|Default|GetPlayerRef)) (Variables|Default|GetCanSpawn))
    (Variables|Default|SetCanSpawn false)
    (Game|SpawnActorfromClass (Variables|EnemiestoSpawn|GetEnemyToSpawn1) (Math|Transform|MakeTransform (Transformation|GetWorldLocation (Variables|Default|GetSpawnPos1)) "0, 0, 0" "1.000000,1.000000,1.000000") "Undefined" "MultiplyWithRoot" 0 0)
    (Variables|Default|SetEnemyRef1 0)))

(event EventBeginPlay
  (bind _asbp_player (Utilities|Casting|CastToBP_Player (Game|GetPlayerCharacter 0)))
  (Variables|Default|SetPlayerRef _asbp_player))

(event Collision|EventActorBeginOverlap
  (params (OtherActor :type Actor%20Object%20Reference)))

(event EventTick
  (params (DeltaSeconds :type Float%20%28single-precision%29)))

(fn ConstructionScript
  (Components|Box|SetBoxExtent (Variables|Default|GetBox) (Variables|Default|GetIn%20Box%20Extent) true)
  (Transformation|SetRelativeLocation (Variables|Default|GetSpawnPos1) (Variables|SpawnLocations|GetSpawn%20Location%201) false false))