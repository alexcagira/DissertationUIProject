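; Shark enemy Blueprint that detects pawns along a line and plays its own death animation, extending a parent enemy class.
; Each tick it traces for Pawn objects from its location to the EndTrace component, with debug drawing, and sets PlayerInRange from the hit result.
; Its OnDeadEvents override runs the parent logic, then stops PaperZD animation overrides and jumps the state machine to DeadJump.
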(event EventBeginPlay
  (|CallParentFunction))

(event Collision|EventActorBeginOverlap
  (params (OtherActor :type Actor%20Object%20Reference))
  (|CallParentFunction OtherActor) ; This node is disabled and will not be called.\nDrag off pins to build functionality.
)

(event EventTick
  (params (DeltaSeconds :type Float%20%28single-precision%29))
  (|CallParentFunction DeltaSeconds)
  (bind _returnvalue (Collision|LineTraceForObjects (Transformation|GetActorLocation) (Transformation|GetWorldLocation (Variables|Default|GetEnd%20Trace)) (Utilities|Array|MakeArray "ObjectTypeQuery3") false 0 "ForOneFrame"))
  (if _returnvalue
    (Variables|Default|SetPlayerInRange true)
    (else
      (Variables|Default|SetPlayerInRange false))))

(fn ConstructionScript
  (|CallParentFunction))

(fn OnDeadEvents
  (bind _paperzdanimation (Variables|Default|GetPaperZDAnimation))
  (bind _animinstance (Variables|/Script/PaperZD.PaperZDAnimationComponent|GetAnimInstance _paperzdanimation))
  (|CallParentFunction)
  (Class|PaperZDAnimInstance|StopAllAnimationOverrides _animinstance)
  (Class|PaperZDAnimInstance|JumptoNode _animinstance "DeadJump" "None"))