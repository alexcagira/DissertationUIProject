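; BP_SharkProjectile is a projectile for the shark enemy that damages the player on contact.
; It caches the player character on BeginPlay, and its Hitbox overlap applies BaseDamage to that player, then destroys the actor.
; Each tick a Visibility line trace runs from the actor to its EndTrace component, drawn for debug, and any hit destroys the projectile without dealing damage.
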(event OnComponentBeginOverlap(Hitbox)
  (params (OverlappedComponent :type Primitive%20Component%20Object%20Reference) (OtherActor :type Actor%20Object%20Reference) (OtherComp :type Primitive%20Component%20Object%20Reference) (OtherBodyIndex :type Integer) (bFromSweep :type Boolean) (SweepResult :type Hit%20Result%20Structure%20%28by%20ref%29))
  (if (== OtherActor (Variables|Default|GetPlayerRef))
    (Game|Damage|ApplyDamage (Variables|Default|GetPlayerRef) (Variables|Default|GetBase%20Damage) 0 0)
    (Actor|DestroyActor)))

(event EventBeginPlay
  (bind _asbp_player (Utilities|Casting|CastToBP_Player (Game|GetPlayerCharacter 0)))
  (Variables|Default|SetPlayerRef _asbp_player))

(event Collision|EventActorBeginOverlap
  (params (OtherActor :type Actor%20Object%20Reference)))

(event EventTick
  (params (DeltaSeconds :type Float%20%28single-precision%29))
  (bind _returnvalue (Collision|LineTraceByChannel (Transformation|GetActorLocation) (Transformation|GetWorldLocation (Variables|Default|GetEnd%20Trace)) "TraceTypeQuery1" false 0 "ForOneFrame"))
  (if _returnvalue
    (Actor|DestroyActor)))

(fn ConstructionScript)