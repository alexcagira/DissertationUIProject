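; BP_MeleeShark is a melee shark enemy animated with PaperZD that extends a parent enemy Blueprint.
; Each tick, a debug-drawn line trace to the EndTrace component sets PlayerInRange when it hits any Pawn object.
; Its hitbox starts disabled, with activate and deactivate functions toggling query collision and box size.
; On death, it clears animation overrides and jumps the state machine to its death node.
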(event EventBeginPlay
  (|CallParentFunction)
  (CallFunction|DeactivateHitbox))

(event Collision|EventActorBeginOverlap
  (params (OtherActor :type Actor%20Object%20Reference))
  (|CallParentFunction OtherActor) ; This node is disabled and will not be called.\nDrag off pins to build functionality.
)

(event EventTick
  (params (DeltaSeconds :type Float%20%28single-precision%29))
  (|CallParentFunction DeltaSeconds)
  (bind _returnvalue (Collision|LineTraceForObjects (Transformation|GetActorLocation) (Transformation|GetWorldLocation (Variables|Components|GetEnd%20Trace)) (Utilities|Array|MakeArray "ObjectTypeQuery3") false 0 "ForOneFrame"))
  (if _returnvalue
    (Variables|Default|SetPlayerInRange true)
    (else
      (Variables|Default|SetPlayerInRange false))))

(fn ConstructionScript
  (|CallParentFunction))

(fn ActivateHitbox
  (bind _hitbox (Variables|Components|GetHitbox))
  (Collision|SetCollisionEnabled _hitbox "QueryOnly")
  (Components|Box|SetBoxExtent _hitbox "40.000000,32.000000,50.000000" true))

(fn DeactivateHitbox
  (bind _hitbox (Variables|Components|GetHitbox))
  (Collision|SetCollisionEnabled _hitbox "NoCollision")
  (Components|Box|SetBoxExtent _hitbox "0, 0, 0" true))

(fn OnDeadEvents
  (bind _paperzdanimation (Variables|Components|GetPaperZDAnimation))
  (bind _animinstance (Variables|/Script/PaperZD.PaperZDAnimationComponent|GetAnimInstance _paperzdanimation))
  (|CallParentFunction)
  (Class|PaperZDAnimInstance|StopAllAnimationOverrides _animinstance)
  (Class|PaperZDAnimInstance|JumptoNode _animinstance "DeadJump" "None"))