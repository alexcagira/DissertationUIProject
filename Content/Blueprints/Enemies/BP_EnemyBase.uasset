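; Base enemy character that tracks health and handles its own death.
; Construction copies max health and damage into current values, and BeginPlay caches a reference to the player.
; AnyDamage lowers health with a floor of zero; at zero the enemy disables capsule collision, detaches its controller and is destroyed after a short delay.
; An empty OnDeadEvents function runs before that delay as a death hook.
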(event EventBeginPlay
  (bind _asbp_player (Utilities|Casting|CastToBP_Player (Game|GetPlayerCharacter 0)))
  (Variables|Default|SetPlayerRef _asbp_player))

(event Collision|EventActorBeginOverlap
  (params (OtherActor :type Actor%20Object%20Reference)))

(event EventTick
  (params (DeltaSeconds :type Float%20%28single-precision%29)))

(event Game|Damage|EventAnyDamage
  (params (Damage :type Float%20%28single-precision%29) (DamageType :type Damage%20Type%20Object%20Reference) (InstigatedBy :type Controller%20Object%20Reference) (DamageCauser :type Actor%20Object%20Reference))
  (bind _output_get (Variables|Default|SetCurrentHealth (Math|Float|Clamp(Float) (- (Variables|Default|GetCurrentHealth) Damage) 0.0 (- (Variables|Default|GetCurrentHealth) Damage))))
  (if (== _output_get 0.0)
    (Variables|Default|SetIsDead true)
    (if (Variables|Default|GetIsDead)
      (Collision|SetCollisionEnabled (Variables|Default|GetCapsuleComponent) "NoCollision")
      (Class|Pawn|DetachfromControllerPendingDestroy)
      (CallFunction|OnDeadEvents)
      (Utilities|FlowControl|Delay 1.0)
      (Actor|DestroyActor))))

(fn ConstructionScript
  (Variables|Default|SetCurrentHealth (Variables|Default|GetMaxHealth))
  (Variables|Default|SetCurrentDamage (Variables|Default|GetMaxDamage)))

(fn OnDeadEvents)