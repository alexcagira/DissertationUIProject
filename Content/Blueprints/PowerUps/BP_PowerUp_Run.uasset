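; BP_PowerUp_Run is a child power-up that temporarily changes the player's walk speed.
; On sphere overlap, it sets PlayerRef's MaxWalkSpeed to PoweredMovement and starts a one-shot timer of PowerUpTimer length, without checking the overlapping actor.
; ResetPlayerWalkSpeed, the likely timer callback, restores NormalMovement and destroys the pickup.
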(event OnComponentBeginOverlap(Sphere)
  (params (OverlappedComponent :type Primitive%20Component%20Object%20Reference) (OtherActor :type Actor%20Object%20Reference) (OtherComp :type Primitive%20Component%20Object%20Reference) (OtherBodyIndex :type Integer) (bFromSweep :type Boolean) (SweepResult :type Hit%20Result%20Structure%20%28by%20ref%29))
  (Variables|/Script/Engine.CharacterMovementComponent|SetMaxWalkSpeed (Variables|/Script/Engine.Character|GetCharacterMovement (Variables|Default|GetPlayerRef)) (Variables|Default|GetPoweredMovement))
  (Utilities|Time|SetTimerbyEvent (EventDispatchers|CreateEvent :!event ResetPlayerWalkSpeed) (Variables|Default|GetPowerUpTimer)))

(event EventBeginPlay
  (|CallParentFunction))

(fn ConstructionScript
  (|CallParentFunction))

(fn ResetPlayerWalkSpeed
  (Variables|/Script/Engine.CharacterMovementComponent|SetMaxWalkSpeed (Variables|/Script/Engine.Character|GetCharacterMovement (Variables|Default|GetPlayerRef)) (Variables|Default|GetNormalMovement))
  (Actor|DestroyActor))